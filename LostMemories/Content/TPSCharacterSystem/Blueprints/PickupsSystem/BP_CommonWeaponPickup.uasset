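; BP_CommonWeaponPickup is a pickup in the TPS character system that carries an existing weapon actor.
; Setting the pickup weapon stores it and attaches it to WeaponMesh, snapping location and keeping relative rotation and scale.
; ServerSetTransferPickupWeaponActor stores a transferred weapon, then attaches it through that setter after a short delay.
; Getters expose both references and the pickup weapon cast to BP_BaseWeapon.
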(event `ServerSetTransferPickupWeaponActor`
  (params (TransferPickupWeaponActor :type "Actor Object Reference"))
  ;[1 1 1] ServerSetTransferPickupWeaponActor
  (`/Engine/EditorBlueprintResources/StandardMacros.IsValid` TransferPickupWeaponActor
    (:`Is Valid`
      (set `self.TransferPickupWeaponActor` TransferPickupWeaponActor)
      (`KismetSystemLibrary.Delay` 0.5)
      (`self.SetPickupWeaponActor` (`self.TransferPickupWeaponActor`)))))

(fn `GetBasePickupWeaponActor`
  (returns (`Base Pickup Weapon` :type "/Game/TPSCharacterSystem/Blueprints/COMMON_WeaponSystem/BP_BaseWeapon Object Reference"))
  (bind _asbp_base_weapon (cast `/Game/TPSCharacterSystem/Blueprints/COMMON_WeaponSystem/BP_BaseWeapon` (`self.PickupWeaponActor`)))
  (return _asbp_base_weapon))

(fn `GetPickupWeaponActor`
  (returns (PickupWeaponActor :type "Actor Object Reference"))
  (return (`self.PickupWeaponActor`)))

(fn `GetTransferPickupWeaponActor`
  (returns (TransferPickupWeaponActor :type "Actor Object Reference"))
  (return (`self.TransferPickupWeaponActor`)))

(fn `SetPickupWeaponActor`
  (params (PickupWeaponActor :type "Actor Object Reference"))
  (`/Engine/EditorBlueprintResources/StandardMacros.IsValid` PickupWeaponActor
    (:`Is Valid`
      (bind _output_get (set `self.PickupWeaponActor` PickupWeaponActor))
      (`self.K2_AttachToComponent` _output_get (`self.WeaponMesh`) "None" "SnapToTarget" "KeepRelative" "KeepRelative" true))))

(fn `SetTransferPickupWeaponActor`
  (params (TransferPickupWeaponActor :type "Actor Object Reference"))
  (`/Engine/EditorBlueprintResources/StandardMacros.IsValid` TransferPickupWeaponActor
    (:`Is Valid`
      (set `self.TransferPickupWeaponActor` TransferPickupWeaponActor))))

(fn `UserConstructionScript`
  (`parent.UserConstructionScript`))