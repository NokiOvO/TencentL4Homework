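; Third-person shooter player character that wires the TPS camera, weapon system and shooting animation controller together.
; On BeginPlay the server spawns primary and secondary weapons and initializes them, while remotes update HUD properties after a delay.
; Weapon swaps and pickups re-attach the hand weapon, reinitialize it and refresh the HUD.
; Character states select camera presets with optional mirroring, and a separate event picks mesh and AnimBP from the GameInstance skin.
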(event `SetMeshAndAnimBlueprint`
  ;[1 1 1] EVENT BEGIN PLAY (ON SPAWN CHARACTER)
  ;;[1 1 1] SetSkeletalMeshAndAnimBluePrint
  (bind _asgame_in_main (cast `/Game/MultiPlayer/Game/GameIN_Main` (`GameplayStatics.GetGameInstance`))
    (:`then`
      (bind (_playerinfo_name _playerinfo_state _playerinfo_ready_ _playerinfo_skin) (break `/Game/MultiPlayer/Game/Variable/Str_PlayerInfo` (`/Game/MultiPlayer/Game/GameIN_Main.PlayerInfo` _asgame_in_main)))
      (switch `string` (`KismetTextLibrary.Conv_TextToString` _playerinfo_skin)
        (:`MHXX`
          (`SkinnedMeshComponent.SetSkinnedAssetAndUpdate` (`self.Mesh`) "/Game/MHXX/Meshes/MHXX_FullClothes.MHXX_FullClothes" true)
          (`SkeletalMeshComponent.SetAnimInstanceClass` (`self.Mesh`) "/Game/MHXX/Blueprint/BP_BASIC_TPSCharacter_MHXX.BP_BASIC_TPSCharacter_MHXX_C"))
        (:`DemonGirl`
          (`SkinnedMeshComponent.SetSkinnedAssetAndUpdate` (`self.Mesh`) "/Game/DaemonGirl/Meshes/DaemonGirl_FullClothes.DaemonGirl_FullClothes" true)
          (`SkeletalMeshComponent.SetAnimInstanceClass` (`self.Mesh`) "/Game/DaemonGirl/Blueprint/BP_BASIC_TPSCharacter_DemonGirl.BP_BASIC_TPSCharacter_DemonGirl_C"))
        (:`Tifa`
          (`SkinnedMeshComponent.SetSkinnedAssetAndUpdate` (`self.Mesh`) "/Game/Tifa/Meshes/Tifa_FullClothes.Tifa_FullClothes" true)
          (`SkeletalMeshComponent.SetAnimInstanceClass` (`self.Mesh`) "/Game/Tifa/Blueprint/BP_BASIC_TPSCharacter_Tifa.BP_BASIC_TPSCharacter_Tifa_C")))
      (`KismetSystemLibrary.PrintString` "Seted." true true (struct :`G` 0.66 :`B` 1.0 :`A` 1.0) 10.0)
      (`KismetSystemLibrary.PrintString` (`KismetSystemLibrary.GetObjectName` (`SkeletalMeshComponent.GetAnimInstance` (`self.Mesh`))) true true (struct :`G` 0.66 :`B` 1.0 :`A` 1.0) 10.0))
    (:`CastFailed`
      (`KismetSystemLibrary.PrintString` "CastFailed" true true (struct :`G` 0.66 :`B` 1.0 :`A` 1.0) 10.0))))

(event `self.ReceiveBeginPlay`
  ;[1 1 1] EVENT BEGIN PLAY (ON SPAWN CHARACTER)
  (`parent.ReceiveBeginPlay`)
  ;;[1 1 1] Initialize TPS Camera
  (`self.InitializeTPSCamera`)
  (`|ExecutionSequence`
    (:`then_0`
      (`/Engine/EditorBlueprintResources/ActorMacros.Switch Has Authority`
        (:`Authority`
          ;;[1 1 1] Spawn Base Weapon as Primary Weapon
          (bind _returnvalue (`|SpawnActorFromClass` (`self.PrimaryWeaponClass`) (`SceneComponent.GetRelativeTransform` (`self.Mesh`)) "AlwaysSpawn" "OverrideRootScale" null null))
          (`/Engine/EditorBlueprintResources/StandardMacros.IsValid` _returnvalue
            (:`Is Valid`
              (`self.Set Primary Weapon Actor` _returnvalue)
              ;;[1 1 1] Spawn Base Weapon as Secondary Weapon
              (bind _returnvalue_2 (`|SpawnActorFromClass` (`self.SecondaryWeaponClass`) (`SceneComponent.GetRelativeTransform` (`self.Mesh`)) "AlwaysSpawn" "OverrideRootScale" null null))
              (`/Engine/EditorBlueprintResources/StandardMacros.IsValid` _returnvalue_2
                (:`Is Valid`
                  (`self.Set Secondary Weapon Actor` _returnvalue_2)
                  ;;[1 1 1] Set Hiden Secondary Weapon & Set Primary Slot in Hand
                  (`self.SetActorHiddenInGame` (`self.Get Secondary Weapon Actor`) false)
                  (`self.Set Current Weapon Slot In Hand` "NewEnumerator0")
                  ;;[1 1 1] Init TPS Weapon
                  (`self.Initialize Basic TPS Weapons`))))))
        (:`Remote`
          ;;[1 1 1] Initialize HUD Properties
          (`KismetSystemLibrary.Delay` 1.0)
          (bind _asbp_basic_wpn_base_weapon (cast `/Game/TPSCharacterSystem/Blueprints/BASIC_BaseCharacter/Data/BP_BASIC_WPN_BaseWeapon` (`self.Get Current Base Weapon`) :!label _label))
          (`self.SetPlayerHUDProperties` (`/Game/TPSCharacterSystem/Blueprints/BASIC_BaseCharacter/Data/BP_BASIC_WPN_BaseWeapon.HUD Properties` _asbp_basic_wpn_base_weapon)))))
    (:`then_1`
      ;;[1 1 1] Wait basic logics
      (`KismetSystemLibrary.Delay` 1.0)
      ;;[1 1 1] Attach Weapon Logic
      (`self.Attach Current Weapon` (`self.Get Current Base Weapon`)))))

(event `ClientUpdateHUDWeaponProp`
  ;[1 1 1] EVENT BEGIN PLAY (ON SPAWN CHARACTER)
  ;;[1 1 1] Initialize HUD Properties
  (goto _label))

(event `InitializeTPSCamera`
  ;[1 1 1] EVENT BEGIN PLAY (ON SPAWN CHARACTER)
  ;;[1 1 1] InitializeTPSCamera
  (`/Engine/EditorBlueprintResources/StandardMacros.IsValid` (`self.BP_AdvancedTPSCamera`)
    (:`Is Valid`
      (`/Engine/EditorBlueprintResources/StandardMacros.IsValid` (`self.SpringArm`)
        (:`Is Valid`
          (`/Engine/EditorBlueprintResources/StandardMacros.IsValid` (`self.Camera`)
            (:`Is Valid`
              (`/Game/TPSCharacterSystem/Blueprints/COMMON_TPSCamera/BP_AdvancedTPSCamera.Set Start Camera Mode` (`self.BP_AdvancedTPSCamera`) (`self.SpringArm`) (`self.Camera`) "FloorIdle" 75.0 -75.0 true))))))))

(event `MulticastAttacthWeapon`
  ;[1 1 1] MulticastAttacthWeapon
  (`self.Attach Current Weapon` (`self.Get Current Base Weapon`))
  (`KismetSystemLibrary.Delay` 0.2)
  (`self.Attach Current Weapon` (`self.Get Current Base Weapon`)))

(event `/Game/TPSCharacterSystem/Blueprints/COMMON_CommonCharacter/BP_CommonCharacterInterface.DeadStateChanged`
  (params (`In Dead?` :type Boolean))
  ;[1 1 1] Event Character State Changed
  (`self.Change Camera State` "Dead"))

(event `UpdateCameraMode`
  (params (`Character State` :type "/Game/TPSCharacterSystem/Blueprints/COMMON_CommonCharacter/ENUM_CharacterState Enum" :default "NewEnumerator0"))
  ;[1 1 1] Event Character State Changed
  (switch `/Game/TPSCharacterSystem/Blueprints/COMMON_CommonCharacter/ENUM_CharacterState` `Character State`
    (:`NewEnumerator0`
      (`self.Change Camera State` "FloorIdle"))
    (:`NewEnumerator1`
      (`self.Change Camera State` "FloorMiniZoom"))
    (:`NewEnumerator2`
      (`self.Change Camera State` "CrouchIdle"))
    (:`NewEnumerator3`
      (`self.Change Camera State` "CrouchMiniZoom"))
    (:`NewEnumerator6`
      (`self.Change Camera State` "FloorSprint"))
    (:`NewEnumerator7`
      (`self.Change Camera State` "CrouchIdle" :!label _label_2))
    (:`NewEnumerator8`
      (goto _label_2))))

(event `/Game/TPSCharacterSystem/Blueprints/COMMON_CommonCharacter/BP_CommonCharacterInterface.SwapTriggerFire`
  ;[1 1 1] Swap
  (`self.MulticastAttacthWeapon` :!label _label_3)
  ;;[1 1 1] Initialize Weapon
  (`self.Initialize Basic TPS Weapons`)
  (`self.ClientUpdateHUDWeaponProp`))

(event `/Game/TPSCharacterSystem/Blueprints/COMMON_CommonCharacter/BP_CommonCharacterInterface.WeaponPickuped`
  ;[1 1 1] Swap
  (goto _label_3))

(event `/Game/TPSCharacterSystem/Blueprints/COMMON_CommonCharacter/BP_CommonCharacterInterface.CharacterStateChanged`
  (params (`Character State` :type "/Game/TPSCharacterSystem/Blueprints/COMMON_CommonCharacter/ENUM_CharacterState Enum" :default "NewEnumerator0"))
  ;[1 1 1] Event Character State Changed
  (`self.UpdateCameraMode` `Character State`))

(event `/Game/TPSCharacterSystem/Blueprints/COMMON_CommonCharacter/BP_CommonCharacterInterface.CameraMirrow`
  ;[1 1 1] Camera Mirror
  (if (`self.In Camera Mirror?`)
    (set `self.In Camera Mirror?` false)
    (else
      (set `self.In Camera Mirror?` true)))
  (`/Game/TPSCharacterSystem/Blueprints/COMMON_TPSCamera/BP_AdvancedTPSCamera.OpenGateChange` (`self.BP_AdvancedTPSCamera`))
  (`self.Change Camera State` (`/Game/TPSCharacterSystem/Blueprints/COMMON_TPSCamera/BP_AdvancedTPSCamera.Current Camera Mode` (`self.BP_AdvancedTPSCamera`))))

(fn `Attach Current Weapon`
  (params (`Current Weapon` :type "Actor Object Reference"))
  (`/Engine/EditorBlueprintResources/StandardMacros.IsValid` `Current Weapon`
    (:`Is Valid`
      (`self.K2_AttachToComponent` `Current Weapon` (`self.Mesh`) "TestWeaponPositionSocket" "SnapToTarget" "KeepRelative" "SnapToTarget" true))))

(fn `Change Camera State`
  (params (`Input Camera Preset` :type Name))
  (`/Game/TPSCharacterSystem/Blueprints/COMMON_TPSCamera/BP_AdvancedTPSCamera.OpenGateChange` (`self.BP_AdvancedTPSCamera`))
  (`/Game/TPSCharacterSystem/Blueprints/COMMON_TPSCamera/BP_AdvancedTPSCamera.Change Camera Mode` (`self.BP_AdvancedTPSCamera`) (`self.SpringArm`) (`self.Camera`) `Input Camera Preset` (`self.In Camera Mirror?`)))

(fn `Initialize Basic TPS Weapons`
  (locals (loc_row :type "/Game/TPSCharacterSystem/Blueprints/BASIC_TPSCharacter/Data/STR_BASIC_TPS_WeaponDecs Structure"))
  ;[0.2017 1 0.05392] WS Set Current Weapon
  (`/Game/TPSCharacterSystem/Blueprints/COMMON_WeaponSystem/BP_WeaponSystem.SetCurrentWeapon` (`self.BP_WeaponSystem`) (`self.Get Current Base Weapon`))
  ;[1 1 1] Initialize basic base settings
  (bind _asbp_basic_wpn_base_weapon (cast `/Game/TPSCharacterSystem/Blueprints/BASIC_BaseCharacter/Data/BP_BASIC_WPN_BaseWeapon` (`self.Get Current Base Weapon`)))
  (bind (_weaponpositioninrighthand _usedefaultreloadanimation_ _newreloadanimationmontage) (break `/Game/TPSCharacterSystem/Blueprints/BASIC_BaseCharacter/Data/STR_BASIC_Weapon3RDPPPropertiesDesc` (`/Game/TPSCharacterSystem/Blueprints/BASIC_BaseCharacter/Data/BP_BASIC_WPN_BaseWeapon.Get3RDPPProperties` _asbp_basic_wpn_base_weapon)))
  (`self.Initialize Basic Base Properties` (`.WeaponAnimType_2_A75BFA7B422FB26C78E0AEB118FABFDD` (break `/Game/TPSCharacterSystem/Blueprints/BASIC_BaseCharacter/Data/STR_BASIC_WeaponCommonPropertiesDesc` (`/Game/TPSCharacterSystem/Blueprints/BASIC_BaseCharacter/Data/BP_BASIC_WPN_BaseWeapon.GetCommonProperties` _asbp_basic_wpn_base_weapon))) _weaponpositioninrighthand _usedefaultreloadanimation_ _newreloadanimationmontage)
  ;[1 1 1] Shooting Animation Controller
  (`/Game/TPSCharacterSystem/Blueprints/COMMON_ShootingAnimationController/BP_ShootingAnimationController.Set3RDPPShootAnimPreset` (`self.BP_ShootingAnimController`) (`/Game/TPSCharacterSystem/Blueprints/COMMON_WeaponSystem/BP_WeaponSystem.GetWeaponFireRate` (`self.BP_WeaponSystem`)) (`/Game/TPSCharacterSystem/Blueprints/BASIC_BaseCharacter/Data/BP_BASIC_WPN_BaseWeapon.Get3RDPPShootingAnimProperties` _asbp_basic_wpn_base_weapon)))

(fn `UserConstructionScript`
  (`parent.UserConstructionScript`))